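; AI controller for the alien that runs BT_Alien and feeds its Blackboard with player detection state.
; Perception updates flag line of sight to the Player-tagged actor, with a timer delaying loss of the enemy.
; Each tick, sight raises or decays an awareness gauge, pushed to BP_Alien, that sets noticed and targeting keys, clearing both only at zero.
; Tick also flags player proximity within the kill zone; EnhanceSenses is an empty stub.
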(event OnTargetPerceptionUpdated(AIPerception)
  (params (Actor :type Actor%20Object%20Reference) (Stimulus :type AI%20Stimulus%20Structure))
  (bind _blackboard (Variables|Default|GetBlackboard))
  (bind _returnvalue (CallFunction|UpdateLineOfSight Actor Stimulus))
  (if _returnvalue
    (Utilities|Time|ClearandInvalidateTimerbyHandle (Variables|Default|GetEnemyTimer))
    (AI|Components|Blackboard|SetValueasBool _blackboard (Variables|Default|GetHasLineOfSight) true)
    (AI|Components|Blackboard|SetValueasObject _blackboard (Variables|Default|GetEnemyActor) Actor)
    (else
      (bind _returnvalue_2 (Utilities|Time|SetTimerbyEvent (delegate Custom|StartEnemyTimer) (Variables|Default|GetLineOfSightTimer)))
      (Variables|Default|SetEnemyTimer _returnvalue_2))))

(event Custom|StartEnemyTimer
  (bind _blackboard (Variables|Default|GetBlackboard))
  (AI|Components|Blackboard|SetValueasBool _blackboard (Variables|Default|GetHasLineOfSight) false)
  (AI|Components|Blackboard|SetValueasObject _blackboard (Variables|Default|GetEnemyActor) 0))

(event EventTick
  (params (DeltaSeconds :type Float%20%28single-precision%29))
  (bind _returnvalue (Game|Player|GetPlayerPawn 0))
  (CallFunction|UpdateIsTargetingPlayer DeltaSeconds)
  (Utilities|IsValid _returnvalue
    (:Is%20Valid
      (CallFunction|UpdateIsWithinKillZone _returnvalue))))

(event EventPossess
  (params (PossessedPawn :type Pawn%20Object%20Reference))
  (AI|RunBehaviorTree "/Game/AI/BT_Alien.BT_Alien"))

(fn ConstructionScript)

(fn UpdateLineOfSight
  (params (self2 :type Actor%20Object%20Reference) (AIStimulus :type AI%20Stimulus%20Structure%20%28by%20ref%29))
  (bind _bsuccessfullysensed (Utilities|Struct|BreakAIStimulus AIStimulus))
  (bind _returnvalue (Actor|ActorHasTag self2 "Player"))
  (bind _returnvalue_2 (and _returnvalue _bsuccessfullysensed))
  (Variables|Default|SetbHasLineOfSight _returnvalue_2)
  (return _returnvalue_2))

(fn UpdateIsTargetingPlayer
  (params (DeltaTime :type Float%20%28double-precision%29))
  (bind _output_get (|UpdatePlayerAwarenessGauge DeltaTime DeltaTime)
    (:then
      _)
    (:then2
      _))
  (bind _returnvalue (Actor|GetActorOfClass "/Game/Blueprints/BP_Alien.BP_Alien_C"))
  (Utilities|IsValid _returnvalue
    (:Is%20Valid
      (Default|SetPlayerTargetingGaugeSliderPercent _returnvalue _output_get)
      (if (> (Variables|Default|GetPlayerAwarenessGauge) 2e+01)
        (AI|Components|Blackboard|SetValueasBool (Variables|Default|GetBlackboard) (Variables|Default|GetHasNoticedPlayer) true))
      ;[1 1 1] Decide if player is being targeted yet based on gauge
      (if (> (Variables|Default|GetPlayerAwarenessGauge) 9e+01)
        (AI|Components|Blackboard|SetValueasBool (Variables|Default|GetBlackboard) (Variables|Default|GetIsTargetingPlayer) true)
        (elif (== (Variables|Default|GetPlayerAwarenessGauge) 0.0)
          (AI|Components|Blackboard|SetValueasBool (Variables|Default|GetBlackboard) (Variables|Default|GetIsTargetingPlayer) false)
          (AI|Components|Blackboard|SetValueasBool (Variables|Default|GetBlackboard) (Variables|Default|GetHasNoticedPlayer) false))))
    (:Is%20Not%20Valid
      (Development|PrintString "Couldn't get BP_Alien in B_AlienController"))))

(fn UpdateIsWithinKillZone
  (params (TargetActor :type Actor%20Object%20Reference))
  (bind _returnvalue (Actor|GetActorOfClass "/Game/Blueprints/BP_Alien.BP_Alien_C"))
  (Utilities|IsValid _returnvalue
    (:Is%20Valid
      (AI|Components|Blackboard|SetValueasBool (Variables|Default|GetBlackboard) (Variables|Default|GetIsWithinKillZone) (< (Transformation|GetDistanceTo TargetActor _returnvalue) (Variables|Default|GetKillZoneRadius))))
    (:Is%20Not%20Valid
      (Development|PrintString "Couldn't get BP_Alien in B_AlienController, Update IsWithinKillZone"))))

(fn EnhanceSenses
  (params (DoEnhance :type Boolean)))