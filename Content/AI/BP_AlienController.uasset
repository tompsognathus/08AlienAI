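; AI controller for an alien that runs the BT_Alien behavior tree and decides when it is targeting the player.
; Perception updates set line of sight to Player-tagged actors and write it, along with the enemy actor, to the Blackboard.
; Each tick, an awareness gauge grows with sight and decays without it, toggling IsTargetingPlayer through high and low thresholds for hysteresis, with debug prints.
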(event OnTargetPerceptionUpdated(AIPerception)
  (params (Actor :type Actor%20Object%20Reference) (Stimulus :type AI%20Stimulus%20Structure))
  (bind _blackboard (Variables|Default|GetBlackboard))
  (bind _blackboard_2 (Variables|Default|GetBlackboard))
  (bind _returnvalue (CallFunction|UpdateLineOfSight Actor Stimulus))
  (if _returnvalue
    (AI|Components|Blackboard|SetValueasBool _blackboard (Variables|Default|GetHasLineOfSight) true)
    (AI|Components|Blackboard|SetValueasObject _blackboard (Variables|Default|GetEnemyActor) Actor)
    (else
      (AI|Components|Blackboard|SetValueasBool _blackboard_2 (Variables|Default|GetHasLineOfSight) false)
      (AI|Components|Blackboard|SetValueasObject _blackboard_2 (Variables|Default|GetEnemyActor) 0))))

(event EventTick
  (params (DeltaSeconds :type Float%20%28single-precision%29))
  (CallFunction|UpdateIsTargetingPlayer DeltaSeconds))

(event EventPossess
  (params (PossessedPawn :type Pawn%20Object%20Reference))
  (AI|RunBehaviorTree "/Game/AI/BT_Alien.BT_Alien"))

(fn ConstructionScript)

(fn UpdateLineOfSight
  (params (self2 :type Actor%20Object%20Reference) (AIStimulus :type AI%20Stimulus%20Structure%20%28by%20ref%29))
  (bind _bsuccessfullysensed (Utilities|Struct|BreakAIStimulus AIStimulus))
  (bind _returnvalue (Actor|ActorHasTag self2 "Player"))
  (bind _returnvalue_2 (and _returnvalue _bsuccessfullysensed))
  (Variables|Default|SetbHasLineOfSight _returnvalue_2)
  (return _returnvalue_2))

(fn UpdateIsTargetingPlayer
  (params (DeltaTime :type Float%20%28double-precision%29))
  (if (Variables|Default|GetbHasLineOfSight)
    (Variables|Default|SetPlayerAwarenessGauge (Math|Float|Min(Float) (+ (Variables|Default|GetPlayerAwarenessGauge) (* (Variables|Default|GetPlayerAwarenessGrowthRate) DeltaTime)) 1e+02))
    (else
      (Variables|Default|SetPlayerAwarenessGauge (Math|Float|Max(Float) (- (Variables|Default|GetPlayerAwarenessGauge) (* DeltaTime (Variables|Default|GetPlayerAwarenessDecayRate))) 0.0))))
  (if (> (Variables|Default|GetPlayerAwarenessGauge) 9e+01)
    (AI|Components|Blackboard|SetValueasBool (Variables|Default|GetBlackboard) (Variables|Default|GetIsTargetingPlayer) true)
    (Development|PrintString "Targeting player")
    (elif (< (Variables|Default|GetPlayerAwarenessGauge) 1e+01)
      (AI|Components|Blackboard|SetValueasBool (Variables|Default|GetBlackboard) (Variables|Default|GetIsTargetingPlayer) false)))
  (Development|PrintString (Utilities|String|ToString(Float) (Variables|Default|GetPlayerAwarenessGauge))))